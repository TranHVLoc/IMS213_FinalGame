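; Alligator hazard actor that travels along a spline path and bites the first-person player on contact.
; On BeginPlay it finds the BP_MovingPath_Bite actor, caches its spline length and starts a timeline.
; The timeline lerps distance along the spline, setting world-space location and local-space rotation each update.
; Overlapping BP_FirstPersonCharacter deducts two from its collected trash count and plays a 2D snap sound.
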(event `self.ReceiveBeginPlay`
  ;[1 1 1] Get reference from external path
  (bind _returnvalue (`GameplayStatics.GetActorOfClass` "/Game/Blueprints/BP_MovingPath_Bite.BP_MovingPath_Bite_C"))
  (set `self.alligatorPathReference` _returnvalue)
  ;[1 1 1] Get the length of that reference path/spline
  (set `self.alligatorPathLength` (`SplineComponent.GetSplineLength` (`/Game/Blueprints/BP_MovingPath_Bite.Spline` (`self.alligatorPathReference`))))
  (`self.playAlligatorTimeLine`))

(event `playAlligatorTimeLine`
  (bind (_direction _alligatormovement) (`Timeline|alligatorTimeline`)
    (:`Update`
      (bind _returnvalue (`KismetMathLibrary.Lerp` 0.0 (`self.alligatorPathLength`) _alligatormovement))
      (`self.K2_SetActorTransform` (`KismetMathLibrary.MakeTransform` (`SplineComponent.GetLocationAtDistanceAlongSpline` (`/Game/Blueprints/BP_MovingPath_Bite.Spline` (`self.alligatorPathReference`)) _returnvalue "World") (`SplineComponent.GetRotationAtDistanceAlongSpline` (`/Game/Blueprints/BP_MovingPath_Bite.Spline` (`self.alligatorPathReference`)) _returnvalue "Local"))))))

(event `self.ReceiveActorBeginOverlap`
  (params (OtherActor :type "Actor Object Reference"))
  (bind _asbp_first_person_character (cast `/Game/FirstPerson/Blueprints/BP_FirstPersonCharacter` OtherActor))
  (set `/Game/FirstPerson/Blueprints/BP_FirstPersonCharacter.myTrashCollected` (- (`/Game/FirstPerson/Blueprints/BP_FirstPersonCharacter.myTrashCollected` _asbp_first_person_character) 2) _asbp_first_person_character)
  (`GameplayStatics.PlaySound2D` "/Game/Assets/CU_Snap.CU_Snap" 1.0 1.0 0.0 null null))

(fn `UserConstructionScript`)